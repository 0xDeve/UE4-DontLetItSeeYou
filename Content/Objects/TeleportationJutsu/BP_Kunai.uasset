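; BP_Kunai is a pickup item whose skill teleports its owner with a teleportation jutsu.
; Pickup runs the parent logic, plays a kunai sound and adds the Kunai_UI widget.
; Activation plays audio, shows the TeleJutsu widget and briefly slows global time before moving the owner to a random TeleportPoints actor.
; The kunai then destroys itself, making the skill single-use.
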(event EventBeginPlay)

(event Collision|EventActorBeginOverlap
  (params (OtherActor :type Actor%20Object%20Reference)))

(event EventTick
  (params (DeltaSeconds :type Float%20%28single-precision%29)))

(event EventActivateSkill
  (|CallParentFunction)
  (Audio|PlaySound2D "/Game/Objects/TeleportationJutsu/jutsu__online-audio-converter_com_.jutsu__online-audio-converter_com_" 1.0 1.0 0.0 0 0)
  (bind _returnvalue (UserInterface|CreateWidget "/Game/Objects/TeleportationJutsu/TeleJutsu.TeleJutsu_C" (Game|GetPlayerController 0)))
  (UserInterface|Viewport|AddtoViewport _returnvalue 0)
  (Utilities|Time|SetGlobalTimeDilation 0.2)
  (Utilities|FlowControl|Delay 0.5)
  (Audio|PlaySound2D "/Game/Objects/TeleportationJutsu/flying.flying" 1.0 1.0 0.0 0 0)
  (Utilities|Time|SetGlobalTimeDilation 1.0)
  (Transformation|SetActorLocation (Components|GetOwner) (Transformation|GetActorLocation (.OutItem (Utilities|Array|Random (Variables|Default|GetTeleportPoints)))) false false)
  (Actor|DestroyActor))

(event EventOnPickup
  (params (InInteractor :type Dont%20Let%20Him%20See%20You%20Character%20Object%20Reference))
  (|CallParentFunction InInteractor)
  (Audio|PlaySoundatLocation "/Game/VFX/Kunai/kunai.kunai" (Transformation|GetActorLocation) "0, 0, 0" 1.0 1.0 0.0 0 0 0 0)
  (bind _returnvalue (UserInterface|CreateWidget "/Game/UI/RaijinJutsu/Kunai_UI.Kunai_UI_C" (Game|GetPlayerController 0)))
  (UserInterface|Viewport|AddtoViewport _returnvalue 0))

(fn ConstructionScript)
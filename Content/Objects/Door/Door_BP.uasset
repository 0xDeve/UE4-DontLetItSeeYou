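; Door Blueprint that swings open with a squeaking sound the first time an actor overlaps it, then swings shut after a short delay.
; The DoorRotation timeline drives the mesh's relative yaw, offset by the actor yaw cached in the Construction Script, and reverses to close.
; A DoOnce with no reset limits the trigger to one use, and the IsPlaying check always passes because the flag is set just before it.
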(event Collision|EventActorBeginOverlap
  (params (OtherActor :type Actor%20Object%20Reference))
  (Utilities|FlowControl|DoOnce false
    (:Completed
      (bind _output_get (Variables|Default|SetisPlaying? true))
      (if _output_get
        (Audio|PlaySoundatLocation "/Game/Objects/Door/Horror_Sound_Effect_-_Squeaking_Door__mp3cut_net_.Horror_Sound_Effect_-_Squeaking_Door__mp3cut_net_" (Transformation|GetWorldLocation (Variables|Debug|GetStaticMeshComponent)))
        (bind _angle (Timeline|DoorRotation Play)
          (:Update
            (Transformation|SetRelativeRotation (Variables|Debug|GetStaticMeshComponent) (Math|Rotator|MakeRotator 0.0 0.0 (+ _angle (Variables|Default|GetDoorYaw))) false false))
          (:Finished
            (Variables|Default|SetisPlaying? false)
            (Utilities|FlowControl|Delay 4.0)
            (Timeline|DoorRotation Reverse)))))))

(fn ConstructionScript
  (Variables|Default|SetDoorYaw (.yaw (Transformation|GetActorRotation))))
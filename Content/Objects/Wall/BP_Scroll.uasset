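; BP_Scroll is a pickup skill scroll that summons an earth jutsu wall in front of its owner.
; On pickup it plays a sound, adds the EarthJutsu_UI widget to the viewport and disables collision on its two meshes.
; Activation plays a jutsu sound, waits briefly, spawns a scaled-up WallBP ahead of and below the owner, then destroys the scroll, making it single-use.
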(event EventBeginPlay)

(event Collision|EventActorBeginOverlap
  (params (OtherActor :type Actor%20Object%20Reference)))

(event EventTick
  (params (DeltaSeconds :type Float%20%28single-precision%29)))

(event EventOnPickup
  (params (InInteractor :type Dont%20Let%20Him%20See%20You%20Character%20Object%20Reference))
  (|CallParentFunction InInteractor)
  (Audio|PlaySound2D "/Game/VFX/WallJutsu/scroll.scroll" 1.0 1.0 0.0 0 0)
  (bind _returnvalue (UserInterface|CreateWidget "/Game/UI/EarthStyle/EarthJutsu_UI.EarthJutsu_UI_C" (Game|GetPlayerController 0)))
  (UserInterface|Viewport|AddtoViewport _returnvalue 0)
  (Collision|SetCollisionEnabled (Variables|Default|GetStaticMesh1) "NoCollision"))

(event EventActivateSkill
  (bind _returnvalue (Components|GetOwner))
  (bind _returnvalue_2 (Transformation|GetActorLocation _returnvalue))
  (bind _returnvalue_3 (Transformation|GetActorForwardVector _returnvalue))
  (bind _returnvalue_4 (* _returnvalue_3 "300.000000,300.000000,300.000000"))
  (bind _returnvalue_5 (+ _returnvalue_2 _returnvalue_4))
  (bind (_x _y _z) (Math|Vector|BreakVector _returnvalue_5))
  (|CallParentFunction)
  (Audio|PlaySound2D "/Game/Objects/TeleportationJutsu/jutsu__online-audio-converter_com_.jutsu__online-audio-converter_com_" 1.0 1.0 0.0 0 0)
  (Utilities|FlowControl|Delay 2.0)
  (Game|SpawnActorfromClass "/Game/Objects/Wall/WallBP.WallBP_C" (Math|Transform|MakeTransform (Math|Vector|MakeVector _x _y (- _z 5e+02)) "0, 0, 0" "2.000000,2.000000,2.000000") "AlwaysSpawn" 0 0)
  (Actor|DestroyActor))

(fn ConstructionScript)
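; BP_SharinganEye is a pickup skill item that grants a single-hit Amaterasu fire attack.
; Pickup plays a sound and shows an acquire widget on top of the parent behavior.
; Activation uses the owning RunnerBP's Pickup line trace; a blocking hit gets attached fire effects and sound, takes damage, and triggers an activation widget.
; The eye destroys itself after a hit, so a missed trace does not consume it.
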(event EventBeginPlay)

(event Collision|EventActorBeginOverlap
  (params (OtherActor :type Actor%20Object%20Reference)))

(event EventTick
  (params (DeltaSeconds :type Float%20%28single-precision%29)))

(event EventActivateSkill
  (bind _returnvalue (Components|GetOwner))
  (bind _returnvalue_2 (Game|GetInstigatorController _returnvalue))
  (bind _asplayer_controller (Utilities|Casting|CastToPlayerController _returnvalue_2))
  (|CallParentFunction)
  (bind _asrunner_bp (Utilities|Casting|CastToRunnerBP _returnvalue))
  (bind _returnvalue_3 (Class|PickupComponent|LineTrace (Variables|/Game/ThirdPersonCPP/Blueprints/RunnerBP.RunnerBP_C|GetPickup _asrunner_bp)))
  (if (.bBlockingHit (Collision|BreakHitResult _returnvalue_3))
    (Effects|SpawnEmitterAttached "/Game/StarterContent/Particles/Amaterasu.Amaterasu" (.HitComponent (Collision|BreakHitResult _returnvalue_3)) (.HitBoneName (Collision|BreakHitResult _returnvalue_3)) "0, 0, 0" "0, 0, 0" "5.000000,5.000000,5.000000" "SnapToTarget")
    (Audio|PlaySound2D "/Game/VFX/Sharingan/Sonido_de_Sasuke-Amaterasu_.Sonido_de_Sasuke-Amaterasu_" 1.0 1.0 0.0 0 0)
    (bind _returnvalue_4 (UserInterface|CreateWidget "/Game/UI/Sharingan/ActivateAmaterasu_UI.ActivateAmaterasu_UI_C" _asplayer_controller))
    (UserInterface|Viewport|AddtoViewport _returnvalue_4 0)
    (Audio|SpawnSoundAttached "/Game/StarterContent/Audio/Fire01_Cue.Fire01_Cue" (.HitComponent (Collision|BreakHitResult _returnvalue_3)) "None" "0, 0, 0" "0, 0, 0" "KeepRelativeOffset" true 1.0 1.0 0.0 0 0)
    (Game|Damage|ApplyDamage (.HitActor (Collision|BreakHitResult _returnvalue_3)) 1e+02 _asplayer_controller self "/Script/Engine.DamageType")
    (Actor|DestroyActor)))

(event EventOnPickup
  (params (InInteractor :type Dont%20Let%20Him%20See%20You%20Character%20Object%20Reference))
  (|CallParentFunction InInteractor)
  (Audio|PlaySound2D "/Game/VFX/Sharingan/Sharingan_Sound_Effect.Sharingan_Sound_Effect" 1.0 1.0 0.0 0 0)
  (bind _returnvalue (UserInterface|CreateWidget "/Game/UI/Sharingan/SharinganAcquire_UI.SharinganAcquire_UI_C"))
  (UserInterface|Viewport|AddtoViewport _returnvalue 0))

(fn ConstructionScript)
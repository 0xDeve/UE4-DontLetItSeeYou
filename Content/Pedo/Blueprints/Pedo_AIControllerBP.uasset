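; AI controller for the Pedo character that detects Runner actors and passes them to its behavior tree.
; On BeginPlay it initializes the PedoData blackboard and runs Pedo_BehaviorTree.
; Successful AI perception of a "Runner"-tagged RunnerBP sets RunnerKey if it is alive and clears it if dead.
; Losing perception leaves the key unchanged, and the stimulus's sense class is not used.
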(event OnTargetPerceptionUpdated(AIPerception)
  (params (Actor :type Actor%20Object%20Reference) (Stimulus :type AI%20Stimulus%20Structure))
  (Class|AIPerceptionSystem|GetSenseClassforStimulus Stimulus)
  (if (Actor|ActorHasTag Actor "Runner")
    (if (.bSuccessfullySensed (Utilities|Struct|BreakAIStimulus Stimulus))
      (bind _asrunner_bp (Utilities|Casting|CastToRunnerBP Actor))
      (if (Default|IsAlive _asrunner_bp)
        (AI|Components|Blackboard|SetValueasObject (Variables|Default|GetBlackboardComp) (Variables|Default|GetRunner%20Key) Actor)
        (else
          (AI|Components|Blackboard|ClearValue (Variables|Default|GetBlackboardComp) (Variables|Default|GetRunner%20Key)))))))

(event EventBeginPlay
  (bind _blackboardcomponent (Class|AIController|UseBlackboard "/Game/Pedo/Behavior/PedoData.PedoData"))
  (Variables|Default|SetBlackboardComp _blackboardcomponent)
  (AI|RunBehaviorTree "/Game/Pedo/Behavior/Pedo_BehaviorTree.Pedo_BehaviorTree"))

(fn ConstructionScript)